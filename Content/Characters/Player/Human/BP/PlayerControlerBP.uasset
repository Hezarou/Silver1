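; Player controller Blueprint for the human player that stores and applies video options.
; On BeginPlay it loads a saved options object, copies its values and calls Adjust events, which map them to console commands, mostly via Lerp.
; SaveGameHandler writes the values back to the save slot and prints the result.
; LoadOptions is empty, and the first-time save and slider-update logic are disconnected.
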(event Custom|Adjust%20EffectsQuality
  ;[1 1 1] VideoSettings
  (Development|ExecuteConsoleCommand (Utilities|String|Append "sg.EffectsQuality " (Utilities|String|ToString(Integer) (Math|Float|Round (Math|Float|Lerp 0.0 3.0 (Variables|VideoSettings|GetEffectsQuality))))) 0))

(event Custom|Adjust%20Brightness
  ;[1 1 1] VideoSettings
  (Development|ExecuteConsoleCommand (Utilities|String|Append "Gamma " (Utilities|String|ToString(Float) (Math|Float|Lerp 0.5 5.0 (Variables|VideoSettings|GetBrightness)))) 0))

(event Custom|Adjust%20Anti-Alliasing
  ;[1 1 1] VideoSettings
  (Development|ExecuteConsoleCommand (Utilities|String|Append "r.PostProcessAAQuality " (Utilities|String|ToString(Integer) (* (Math|Float|Round (Math|Float|Lerp 0.0 3.0 (Variables|VideoSettings|GetAnti-Alliasing))) 2))) 0))

(event Custom|SaveGameHandler
  (bind _optionsave (Variables|VideoSettings|GetOptionSave))
  ;[1 1 1] Save Options
  (Variables|/Game/GUI/Options/Save.Save_C|SetResloutionScale _optionsave (Variables|VideoSettings|GetResolutionScale))
  (Variables|/Game/GUI/Options/Save.Save_C|SetPostProcessing _optionsave (Variables|VideoSettings|GetPostProcessing))
  (Variables|/Game/GUI/Options/Save.Save_C|SetShadowQuality _optionsave (Variables|VideoSettings|GetShadowQuality))
  (Variables|/Game/GUI/Options/Save.Save_C|SetAnti-Alliasing _optionsave (Variables|VideoSettings|GetAnti-Alliasing))
  (Variables|/Game/GUI/Options/Save.Save_C|SetViewDistance _optionsave (Variables|VideoSettings|GetViewDistance))
  (Variables|/Game/GUI/Options/Save.Save_C|SetBrightness _optionsave (Variables|VideoSettings|GetBrightness))
  (Variables|/Game/GUI/Options/Save.Save_C|SetEffectsQuality _optionsave (Variables|VideoSettings|GetEffectsQuality))
  (bind _returnvalue (SaveGame|SaveGametoSlot _optionsave (Variables|Default|GetOptionsSave)))
  (if _returnvalue
    (Development|PrintString "Options Saved!" true true "(R=0.000000,G=0.948000,B=0.010000,A=1.000000)" 5.0)
    (else
      (Development|PrintString "Options Did not save properly!" true true "(R=0.000000,G=0.948000,B=0.010000,A=1.000000)" 5.0))))

(event Custom|Adjust%20ViewDistance
  ;[1 1 1] VideoSettings
  (Development|ExecuteConsoleCommand (Utilities|String|Append "r.ViewDistanceScale " (Utilities|String|ToString(Float) (Variables|VideoSettings|GetViewDistance))) 0))

(event Custom|Adjust%20ResolutionScale
  ;[1 1 1] VideoSettings
  (Development|ExecuteConsoleCommand (Utilities|String|Append "r.ScreenPercentage " (Utilities|String|ToString(Integer) (Math|Float|Round (Math|Float|Lerp 1e+01 1e+02 (Variables|VideoSettings|GetResolutionScale))))) 0))

(event Custom|Adjust%20PostProssesing
  ;[1 1 1] VideoSettings
  (Development|ExecuteConsoleCommand (Utilities|String|Append "sg.PostProcessQuality " (Utilities|String|ToString(Integer) (Math|Float|Round (Math|Float|Lerp 0.0 3.0 (Variables|VideoSettings|GetPostProcessing))))) 0))

(event Custom|Adjust%20ShadowQuality
  ;[1 1 1] VideoSettings
  (Development|ExecuteConsoleCommand (Utilities|String|Append "sg.ShadowQuality " (Utilities|String|ToString(Integer) (Math|Float|Round (Math|Float|Lerp 0.0 3.0 (Variables|VideoSettings|GetShadowQuality))))) 0))

(event EventBeginPlay
  ;[1 1 1] Options Save Handler
  (bind _returnvalue (SaveGame|DoesSaveGameExist "Options"))
  (if _returnvalue
    (bind _returnvalue_2 (SaveGame|LoadGamefromSlot (Variables|Default|GetOptionsSave)))
    (bind _assave (Utilities|Casting|CastToSave _returnvalue_2))
    (Variables|VideoSettings|SetOptionSave _assave)
    (Variables|VideoSettings|SetBrightness (Variables|/Game/GUI/Options/Save.Save_C|GetBrightness (Variables|VideoSettings|GetOptionSave)))
    (Variables|VideoSettings|SetPostProcessing (Variables|/Game/GUI/Options/Save.Save_C|GetPostProcessing (Variables|VideoSettings|GetOptionSave)))
    (Variables|VideoSettings|SetShadowQuality (Variables|/Game/GUI/Options/Save.Save_C|GetShadowQuality (Variables|VideoSettings|GetOptionSave)))
    (Variables|VideoSettings|SetAnti-Alliasing (Variables|/Game/GUI/Options/Save.Save_C|GetAnti-Alliasing (Variables|VideoSettings|GetOptionSave)))
    (Variables|VideoSettings|SetViewDistance (Variables|/Game/GUI/Options/Save.Save_C|GetViewDistance (Variables|VideoSettings|GetOptionSave)))
    (Variables|VideoSettings|SetEffectsQuality (Variables|/Game/GUI/Options/Save.Save_C|GetEffectsQuality (Variables|VideoSettings|GetOptionSave)))
    (Variables|VideoSettings|SetResolutionScale (Variables|/Game/GUI/Options/Save.Save_C|GetResloutionScale (Variables|VideoSettings|GetOptionSave)))
    (CallFunction|AdjustAnti-Alliasing)
    (CallFunction|AdjustBrightness)
    (CallFunction|AdjustEffectsQuality)
    (CallFunction|AdjustPostProssesing)
    (CallFunction|AdjustResolutionScale)
    (CallFunction|AdjustShadowQuality)
    (CallFunction|AdjustViewDistance)
    (else
      (bind _returnvalue_3 (SaveGame|CreateSaveGameObject)))))

(fn ConstructionScript)

(fn LoadOptions)